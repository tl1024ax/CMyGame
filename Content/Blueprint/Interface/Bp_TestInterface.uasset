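; Test Blueprint that exercises what its debug strings name as IReactToTriggerInterface, a set of trigger-reaction methods.
; BeginPlay calls SteppedToTrigger, BumpTntoToTrigger, Test2 and TouchedToTrigger directly on itself, with no trigger involved.
; Each implementation only prints a debug string.
; SteppedToTrigger is a function graph because it returns a value (always false), while the other three are events.
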(event EventBeginPlay
  (CallFunction|SteppedtoTrigger)
  (Class|ReacttoTriggerInterface|BumpTntotoTrigger)
  (Class|ReacttoTriggerInterface|Test2 99)
  (Class|ReacttoTriggerInterface|TouchedtoTrigger))

(event EventTest2
  (params (gold :type Integer))
  (Development|PrintString "BP-IReactToTriggerInterface::Test_2" true true "(R=0.000000,G=0.660000,B=1.000000,A=1.000000)" 12.0))

(event EventBumpTntotoTrigger
  (Development|PrintString "BP-IReactToTriggerInterface::BumpTntoToTrigger" true true "(R=0.000000,G=0.660000,B=1.000000,A=1.000000)" 12.0))

(event EventTouchedtoTrigger
  (Development|PrintString "BP-IReactToTriggerInterface::TouchedToTrigger" true true "(R=0.000000,G=0.660000,B=1.000000,A=1.000000)" 12.0))

(fn ConstructionScript)

(fn SteppedtoTrigger
  (Development|PrintString "BP-IReactToTriggerInterface::ReactToTrigger" true true "(R=0.000000,G=0.660000,B=1.000000,A=1.000000)" 12.0)
  (return false))